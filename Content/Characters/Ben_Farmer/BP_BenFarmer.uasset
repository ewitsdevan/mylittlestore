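; Ben, an AI farmer NPC that harvests crops, carries them and hands them to the player on overlap.
; An event-driven loop uses AIMoveTo to visit harvestable plots until full, then go to the nearest delivery box (once upgraded) or barn.
; HarvestCrop, triggered externally, tallies yields and restarts the loop through CheckAmount.
; Player proximity pauses him and shows a bubble; Interact opens his UI, while Tick drives flipbook, facing and footsteps.
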(event `BenWalkSFX`
  (bind _returnvalue (`PaperFlipbookComponent.GetPlaybackPositionInFrames` (`self.Sprite`)))
  ;[1 1 1] Walk SFX
  (if (or (== _returnvalue 2) (== _returnvalue 6))
    (`KismetSystemLibrary.Delay` 0.1)
    (`GameplayStatics.PlaySoundAtLocation` "/Game/Audio/SFX/CUES/Walking_CUE.Walking_CUE" (`self.K2_GetActorLocation` self) (struct) 1.0 1.0 0.0 null null null)))

(event `self.ReceiveTick`
  (params (DeltaSeconds :type "Float (single-precision)"))
  (bind (_returnvalue_roll _returnvalue_pitch _returnvalue_yaw) (`KismetMathLibrary.BreakRotator` (`KismetMathLibrary.FindLookAtRotation` (`self.K2_GetActorLocation`) (`self.MoveToLocation`))))
  ;[1 1 1] Walk Animation
  (if (`self.isHarvesting`)
    _
    (elif (`self.isMoving`)
      (`PaperFlipbookComponent.SetFlipbook` (`self.Sprite`) "/Game/Characters/Ben_Farmer/Animations/Ben_Walk.Ben_Walk")
      (`self.BenWalkSFX`)
      (if (!= _returnvalue_yaw 0.0)
        (`SceneComponent.K2_SetRelativeRotation` (`self.Sprite`) (`KismetMathLibrary.SelectRotator` (struct :`Yaw` 90.0 :`Roll` -42.5) (struct :`Yaw` 270.0 :`Roll` 42.5) (> _returnvalue_yaw 0.0)) false false))
      (else
        (`PaperFlipbookComponent.SetFlipbook` (`self.Sprite`) "/Game/Characters/Ben_Farmer/Animations/Ben_Idle.Ben_Idle")))))

(event `Pick Up`
  ;[1 1 1] Pickup Animation
  (set `self.isHarvesting` true)
  (`PaperFlipbookComponent.SetFlipbook` (`self.Sprite`) "/Game/Characters/Ben_Farmer/Animations/Ben_PickingUp.Ben_PickingUp")
  (`KismetSystemLibrary.Delay` 1.5)
  (`PaperFlipbookComponent.SetFlipbook` (`self.Sprite`) "/Game/Characters/Ben_Farmer/Animations/Ben_Idle.Ben_Idle")
  (set `self.isHarvesting` false))

(event `ResetItems`
  ;[1 1 1] Reset Item Count
  (set `self.lettuceAmount` 0)
  (set `self.tomatoAmount` 0)
  (set `self.carrotAmount` 0)
  (set `self.hasItems` false)
  (`self.CheckAmount`))

(event `HarvestCrop`
  (params (isLettuce :type Boolean) (isTomato :type Boolean) (isCarrot :type Boolean))
  ;[1 1 1] Harvest Crop
  (`self.Pick Up`)
  (if isLettuce
    (set `self.lettuceAmount` (+ (`self.lettuceAmount`) (`self.harvestYield`)))
    (set `self.hasItems` true)
    (`self.CheckAmount` :!label _label)
    (elif isTomato
      (set `self.tomatoAmount` (+ (`self.tomatoAmount`) (`self.harvestYield`)))
      (set `self.hasItems` true)
      (goto _label)
      (elif isCarrot
        (set `self.carrotAmount` (+ (`self.carrotAmount`) (`self.harvestYield`)))
        (set `self.hasItems` true)
        (goto _label)))))

(event `self.Collider.OnComponentBeginOverlap`
  (params (OverlappedComponent :type "PrimitiveComponent Object Reference") (OtherActor :type "Actor Object Reference") (OtherComp :type "PrimitiveComponent Object Reference") (OtherBodyIndex :type Integer) (bFromSweep :type Boolean) (SweepResult :type "HitResult Structure (by ref)"))
  ;[1 1 1] Player Collect
  (set `self.Other Actor` OtherActor)
  (if (`self.hasItems`)
    (if (`KismetMathLibrary.ClassIsChildOf` (`GameplayStatics.GetObjectClass` (`self.Other Actor`)) "/Game/Characters/Player/BP_Player.BP_Player_C")
      (bind _asbp_player (cast `/Game/Characters/Player/BP_Player` (`self.Other Actor`)))
      (`/Game/Characters/Player/BP_Player.CollectDelivery` _asbp_player (`self.lettuceAmount`) (`self.tomatoAmount`) (`self.carrotAmount`) 0)
      (`KismetSystemLibrary.PrintString` "[BenFarmer] Player Collected" true true (struct :`R` 0.25 :`G` 1.0 :`B` 0.5 :`A` 1.0))
      (`self.ResetItems`))))

(event `self.ReceiveBeginPlay`
  (if (`self.canHarvest`)
    (set `self.StartLocation` (`self.K2_GetActorLocation`))
    (set `self.Player` (`GameplayStatics.GetPlayerPawn` 0))
    (bind _outactors (`GameplayStatics.GetAllActorsOfClass` "/Game/Interactables/BP_FarmPlot.BP_FarmPlot_C"))
    (set `self.PlotArray` _outactors)
    (`self.WalkToPlot`)))

(event `WalkToPlot`
  (bind _output (`|GetArrayItem` (`self.PlotArray`) (`self.plotIndex`)))
  ;[1 1 1] AI MoveTo FarmPlot
  (if (not (`self.isPlayerInteracting`))
    (set `self.isMoving` true)
    (set `self.plotBP` _output)
    (if (`/Game/Interactables/BP_FarmPlot.isHarvestable` _output)
      (bind _output_get (set `self.MoveToLocation` (`SceneComponent.K2_GetComponentLocation` (`/Game/Interactables/BP_FarmPlot.TriggerBox` (`self.plotBP`)))))
      (`|AIMoveTo` self _output_get null 1.0
        (:`OnSuccess`
          (set `self.isMoving` false))
        (:`OnFail`
          (set `self.isMoving` false)
          (`self.NextPlot`)))
      (else
        (set `self.isMoving` false)
        (`self.NextPlot`)))))

(event `self.PlayerINTCollider.OnComponentBeginOverlap`
  (params (OverlappedComponent :type "PrimitiveComponent Object Reference") (OtherActor :type "Actor Object Reference") (OtherComp :type "PrimitiveComponent Object Reference") (OtherBodyIndex :type Integer) (bFromSweep :type Boolean) (SweepResult :type "HitResult Structure (by ref)"))
  ;[1 1 1] Interaction Bubble IN/OUT
  (bind _asbp_player (cast `/Game/Characters/Player/BP_Player` OtherActor))
  (bind _output_get (set `self.Player` _asbp_player))
  (bind _asbubble_int (cast `/Game/UI/Dialogue/Bubble_INT` (`WidgetComponent.GetWidget` (`self.DialogueBubble`))))
  (`/Game/UI/Dialogue/Bubble_INT.Interact_Bubble_IN` _asbubble_int)
  (set `self.isPlayerInteracting` true)
  (bind (_returnvalue_roll _returnvalue_pitch _returnvalue_yaw) (`KismetMathLibrary.BreakRotator` (`KismetMathLibrary.FindLookAtRotation` (`self.K2_GetActorLocation`) (`self.K2_GetActorLocation` _output_get))))
  (if (!= _returnvalue_yaw 0.0)
    (`SceneComponent.K2_SetRelativeRotation` (`self.Sprite`) (`KismetMathLibrary.SelectRotator` (struct :`Yaw` 90.0 :`Roll` -42.5) (struct :`Yaw` 270.0 :`Roll` 42.5) (> _returnvalue_yaw 0.0)) false false)
    (`GameplayStatics.PlaySoundAtLocation` "/Game/Audio/SFX/CUES/Dialogue_CUE.Dialogue_CUE" (`self.K2_GetActorLocation` self) (struct) 1.0 1.0 0.0 null null null)
    (`MovementComponent.StopMovementImmediately` (`self.CharacterMovement`))))

(event `NextPlot`
  ;[1 1 1] Select Next Harvestable Plot
  (for (_array_element _array_index) (`self.PlotArray`)
    (bind _output_get (set `self.plotBP` _array_element))
    (set `self.plotIndex` _array_index)
    (if (`/Game/Interactables/BP_FarmPlot.isUnlocked` _output_get)
      (if (`/Game/Interactables/BP_FarmPlot.isHarvestable` (`self.plotBP`))
        (break))))
  (if (`/Game/Interactables/BP_FarmPlot.isHarvestable` (`self.plotBP`))
    (`self.WalkToPlot`)
    (else
      (`self.WalkToBarn`))))

(event `Deliver`
  ;[1 1 1] AI MoveTo DeliveryBox
  (if (not (`self.isPlayerInteracting`))
    (set `self.isMoving` true)
    (bind _outactors (`GameplayStatics.GetAllActorsOfClass` "/Game/Interactables/BP_DeliveryBox.BP_DeliveryBox_C"))
    (bind _output_get (set `self.MoveToLocation` (`self.K2_GetActorLocation` (`.ReturnValue` (`GameplayStatics.FindNearestActor` (`self.K2_GetActorLocation`) _outactors)))))
    (`|AIMoveTo` self _output_get null 1.0
      (:`OnSuccess`
        (set `self.isMoving` false))
      (:`OnFail`
        (set `self.isMoving` false)
        (`self.CheckAmount`)))))

(event `self.PlayerINTCollider.OnComponentEndOverlap`
  (params (OverlappedComponent :type "PrimitiveComponent Object Reference") (OtherActor :type "Actor Object Reference") (OtherComp :type "PrimitiveComponent Object Reference") (OtherBodyIndex :type Integer))
  ;[1 1 1] Interaction Bubble IN/OUT
  (bind _asbp_player (cast `/Game/Characters/Player/BP_Player` OtherActor))
  (set `self.Player` _asbp_player)
  (bind _asbubble_int (cast `/Game/UI/Dialogue/Bubble_INT` (`WidgetComponent.GetWidget` (`self.DialogueBubble`))))
  (`/Game/UI/Dialogue/Bubble_INT.Interact_Bubble_Out` _asbubble_int)
  (set `self.isPlayerInteracting` false)
  (`self.CheckAmount`))

(event `TryAgainDelay`
  ;[1 1 1] Delay Try Again
  (`KismetSystemLibrary.Delay` (`/Game/Interactables/BP_FarmPlot.growTime` (`self.plotBP`)))
  (`self.CheckAmount`))

(event `WalkToBarn`
  (bind _startlocation (`self.StartLocation`))
  ;[1 1 1] AI MoveTo Barn
  (if (not (`self.isPlayerInteracting`))
    (set `self.isMoving` true)
    (set `self.MoveToLocation` _startlocation)
    (`|AIMoveTo` self _startlocation null 1.0
      (:`OnSuccess`
        (set `self.isMoving` false)
        (`self.TryAgainDelay`))
      (:`OnFail`
        (set `self.isMoving` false)
        (`self.CheckAmount`)))))

(event `UI Interact`
  (bind _benwidget (`self.BenWidget`))
  (bind _benwidget_2 (`self.BenWidget`))
  ;[1 1 1] Interact UI
  (bind _asbp_player (cast `/Game/Characters/Player/BP_Player` (`self.Player`)))
  (if (not (`/Game/Characters/Player/BP_Player.isInteracting` _asbp_player))
    (bind _asbubble_int (cast `/Game/UI/Dialogue/Bubble_INT` (`WidgetComponent.GetWidget` (`self.DialogueBubble`))))
    (`/Game/UI/Dialogue/Bubble_INT.Interact_Bubble_Out` _asbubble_int)
    (`/Engine/EditorBlueprintResources/StandardMacros.IsValid` _benwidget_2
      (:`Is Valid`
        (`/Game/UI/Dialogue/BEN_Widget.ShowUI` _benwidget_2))
      (:`Is Not Valid`
        (bind _returnvalue (`|CreateWidget` "/Game/UI/Dialogue/BEN_Widget.BEN_Widget_C" (`GameplayStatics.GetPlayerController` 0)))
        (bind _output_get (set `self.BenWidget` _returnvalue))
        (`UserWidget.AddToViewport` _output_get 0)
        (`/Game/UI/Dialogue/BEN_Widget.ShowUI` _benwidget)))
    (bind _asbp_player_2 (cast `/Game/Characters/Player/BP_Player` (`self.Player`)))
    (set `/Game/Characters/Player/BP_Player.isInteracting` true _asbp_player_2)
    (add `/Game/UI/Dialogue/BEN_Widget.PlayerNotInteracting` _benwidget (delegate `PlayerCanMoveAgain`))
    (add `/Game/UI/Dialogue/BEN_Widget.DeliveryUPGRADE` _returnvalue (delegate `BenCanDeliver`))))

(event `PlayerCanMoveAgain`
  ;[1 1 1] Interact UI
  (set `/Game/Characters/Player/BP_Player.isInteracting` false (stale `UI Interact` _asbp_player_2)))

(event `BenCanDeliver`
  ;[1 1 1] Interact UI
  (set `self.canDeliver` true))

(event `CheckAmount`
  ;[1 1 1] Check Amount
  (bind _output_get (set `self.itemsTotal` (+ (`self.lettuceAmount`) (`self.tomatoAmount`) (`self.carrotAmount`))))
  (`/Engine/EditorBlueprintResources/StandardMacros.CompareInt` _output_get (`self.maxItems`)
    (:`>`
      (if (`self.canDeliver`) :!label _label_2
        (`self.Deliver`)
        (else
          (`self.WalkToBarn`))))
    (:`==`
      (goto _label_2))
    (:`<`
      (`KismetSystemLibrary.Delay` (`self.harvestDelay`))
      (`self.WalkToPlot`))))

(fn `Interact`
  (params (Player :type "/Game/Characters/Player/BP_Player Object Reference"))
  (returns (Success :type Boolean))
  (`self.UI Interact`)
  (return true))

(fn `UserConstructionScript`)