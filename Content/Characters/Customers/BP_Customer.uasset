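; BP_Customer is a shopper AI with a randomly chosen flipbook sprite that walks into the shop, browses and takes stock.
; Chained AI MoveTo events visit random fridges or shelves, randomly pick up fish or vegetables, then head to the till, or the despawner if empty-handed.
; Tick swaps idle/walk flipbooks and flips the sprite by travel direction.
; Failed moves retry, and repeated failures destroy the customer and request a replacement from the spawner.
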(event `self.ReceiveTick`
  (params (DeltaSeconds :type "Float (single-precision)"))
  (bind (_returnvalue_roll _returnvalue_pitch _returnvalue_yaw) (`KismetMathLibrary.BreakRotator` (`KismetMathLibrary.FindLookAtRotation` (`self.K2_GetActorLocation`) (`self.MoveToLocation`))))
  ;[1 1 1] Walk Animation
  (if (`self.isMoving`)
    (`PaperFlipbookComponent.SetFlipbook` (`self.Sprite`) (`|GetArrayItem` (`|MakeArray` "/Game/Characters/Customers/Customer1/Customer1_Walk.Customer1_Walk" "/Game/Characters/Customers/Customer2/Customer2_Walk.Customer2_Walk" "/Game/Characters/Customers/Customer3/Customer3_Walk.Customer3_Walk" "/Game/Characters/Customers/Customer4/Customer4_Walk.Customer4_Walk" "/Game/Characters/Customers/Customer5/Customer5.Customer5" :!type "PaperFlipbook Object Reference") (`self.customerType`)))
    (if (!= _returnvalue_yaw 0.0)
      (`SceneComponent.K2_SetRelativeRotation` (`self.Sprite`) (`KismetMathLibrary.SelectRotator` (struct :`Yaw` 90.0 :`Roll` -42.5) (struct :`Yaw` 270.0 :`Roll` 42.5) (> _returnvalue_yaw 0.0)) false false))
    (else
      (`PaperFlipbookComponent.SetFlipbook` (`self.Sprite`) (`|GetArrayItem` (`|MakeArray` "/Game/Characters/Customers/Customer1/Customer1_Idle.Customer1_Idle" "/Game/Characters/Customers/Customer2/Customer2_Idle.Customer2_Idle" "/Game/Characters/Customers/Customer3/Customer3_Idle.Customer3_Idle" "/Game/Characters/Customers/Customer4/Customer4_Idle.Customer4_Idle" "/Game/Characters/Customers/Customer5/Customer5_Idle.Customer5_Idle" :!type "PaperFlipbook Object Reference") (`self.customerType`))))))

(event `self.ReceiveBeginPlay`
  ;[1 1 1] Set Customer Sprite
  (set `self.customerType` (`KismetMathLibrary.RandomIntegerInRange` 0 4))
  (`PaperFlipbookComponent.SetFlipbook` (`self.Sprite`) (`|GetArrayItem` (`|MakeArray` "/Game/Characters/Customers/Customer1/Customer1_Idle.Customer1_Idle" "/Game/Characters/Customers/Customer2/Customer2_Idle.Customer2_Idle" "/Game/Characters/Customers/Customer3/Customer3_Idle.Customer3_Idle" "/Game/Characters/Customers/Customer4/Customer4_Idle.Customer4_Idle" "/Game/Characters/Customers/Customer5/Customer5_Idle.Customer5_Idle" :!type "PaperFlipbook Object Reference") (`self.customerType`)))
  (`self.WalkToShop`))

(event `AI MoveTo Failed`
  ;[1 1 1] AI MoveTo Failed [Failsafe]
  (`KismetSystemLibrary.PrintString` "[BP_Customer] AI MoveTo Failed")
  (bind _output_get (set `self.timesFailed` (+ (`self.timesFailed`) 1)))
  (`/Engine/EditorBlueprintResources/StandardMacros.CompareInt` _output_get 10
    (:`>`
      _)
    (:`==`
      _))
  (`self.AI Stuck`))

(event `AI Stuck`
  ;[1 1 1] Despawn Actor If Stuck On AI MoveTo Fail [Failsafe]
  (`KismetSystemLibrary.PrintString` "[BP_Customer] AI Stuck")
  (bind _returnvalue (`GameplayStatics.GetActorOfClass` "/Game/Characters/Customers/BP_CustomerSpawner.BP_CustomerSpawner_C"))
  (`/Game/Characters/Customers/BP_CustomerSpawner.SpawnCustomer` _returnvalue)
  (`self.K2_DestroyActor`))

(event `WalkToShop`
  ;[1 1 1] AI MoveTo Shop
  (set `self.isMoving` true)
  (bind _outactors (`GameplayStatics.GetAllActorsOfClass` "/Game/Meshes/Shop_BP.Shop_BP_C"))
  (bind _output_get (set `self.MoveToLocation` (`self.K2_GetActorLocation` (`.ReturnValue` (`GameplayStatics.FindNearestActor` (`self.K2_GetActorLocation`) _outactors)))))
  (`|AIMoveTo` self _output_get null
    (:`OnSuccess`
      (`self.PickShelf`))
    (:`OnFail`
      (`self.WalkToShop`)
      (`self.AI MoveTo Failed`))))

(event `PickShelf`
  ;[1 1 1] Pick Shelf & AI MoveTo Shelf
  (set `self.shelvesChecked` (+ (`self.shelvesChecked`) 1))
  (set `self.isMoving` true)
  (bind _output_get (set `self.getFish` (`KismetMathLibrary.RandomBool`)))
  (if _output_get
    (bind _outactors (`GameplayStatics.GetAllActorsOfClass` "/Game/Interactables/BP_Fridge.BP_Fridge_C"))
    (bind _outitem (`KismetArrayLibrary.Array_Random` _outactors))
    (set `self.fridgeBP` _outitem)
    (bind _output_get_2 (set `self.MoveToLocation` (`self.K2_GetActorLocation` _outitem)))
    (`|AIMoveTo` self _output_get_2 null
      (:`OnSuccess`
        (`self.DecideToPickup`))
      (:`OnFail`
        (`self.PickAnother`)
        (`self.AI MoveTo Failed`)))
    (else
      (bind _outactors_2 (`GameplayStatics.GetAllActorsOfClass` "/Game/Interactables/BP_Shelf.BP_Shelf_C"))
      (bind _outitem_2 (`KismetArrayLibrary.Array_Random` _outactors_2))
      (set `self.shelfBP` _outitem_2)
      (bind _output_get_3 (set `self.MoveToLocation` (`self.K2_GetActorLocation` _outitem_2)))
      (`|AIMoveTo` self _output_get_3 null
        (:`OnSuccess`
          (`self.DecideToPickup`))
        (:`OnFail`
          (`self.PickAnother`)
          (`self.AI MoveTo Failed`))))))

(event `PickAnother`
  ;[1 1 1] Pick Another Shelf [Failsafe]
  (set `self.isMoving` false)
  (`/Engine/EditorBlueprintResources/StandardMacros.CompareInt` (`self.shelvesChecked`) 3
    (:`>`
      (`self.Leave` :!label _label))
    (:`==`
      (goto _label))
    (:`<`
      (`self.PickShelf`))))

(event `DecideToPickup`
  ;[1 1 1] Random Pickup Decision
  (set `self.isMoving` false)
  (`KismetSystemLibrary.Delay` (`self.decisionDelay`))
  (if (`KismetMathLibrary.RandomBool`)
    (`self.PickupItem`)
    (else
      (`self.PickAnother`))))

(event `DecideMore`
  ;[1 1 1] Decide To Pickup More
  (`/Engine/EditorBlueprintResources/StandardMacros.CompareInt` (`self.itemsHeld`) (`self.maxItems`)
    (:`>`
      (`self.Checkout` :!label _label_2))
    (:`==`
      (goto _label_2))
    (:`<`
      (if (`KismetMathLibrary.RandomBool`)
        (`self.PickAnother`)
        (else
          (`self.Checkout`))))))

(event `PickupItem`
  (bind _shelfbp (`self.shelfBP`))
  (bind _fridgebp (`self.fridgeBP`))
  (bind _shelfbp_2 (`self.shelfBP`))
  ;[1 1 1] Pickup Item
  (set `self.isMoving` false)
  (if (`self.getFish`)
    (`/Engine/EditorBlueprintResources/StandardMacros.CompareInt` (`/Game/Interactables/BP_Fridge.stockAmount` (`self.fridgeBP`))
      (:`>`
        (set `/Game/Interactables/BP_Fridge.stockAmount` (- (`/Game/Interactables/BP_Fridge.stockAmount` _fridgebp) 1) _fridgebp)
        (set `self.fishAmount` (+ (`self.fishAmount`) 1))
        (set `self.itemsHeld` (+ (`self.itemsHeld`) 1))
        (`/Game/Interactables/BP_Fridge.UpdateAmount` (`self.fridgeBP`))
        (`self.DecideMore` :!label _label_3))
      (:`==`
        (`self.PickAnother` :!label _label_4))
      (:`<`
        (goto _label_4)))
    (else
      (`/Engine/EditorBlueprintResources/StandardMacros.CompareInt` (`/Game/Interactables/BP_Shelf.stockAmount` (`self.shelfBP`))
        (:`>`
          (set `/Game/Interactables/BP_Shelf.stockAmount` (- (`/Game/Interactables/BP_Shelf.stockAmount` _shelfbp) 1) _shelfbp)
          (if (`/Game/Interactables/BP_Shelf.isCarrot` _shelfbp_2)
            (set `self.carrotAmount` (+ (`self.carrotAmount`) 1))
            (set `self.itemsHeld` (+ (`self.itemsHeld`) 1))
            (`/Game/Interactables/BP_Shelf.UpdateAmount` (`self.shelfBP`))
            (goto _label_3)
            (elif (`/Game/Interactables/BP_Shelf.isLettuce` _shelfbp_2)
              (set `self.lettuceAmount` (+ (`self.lettuceAmount`) 1))
              (set `self.itemsHeld` (+ (`self.itemsHeld`) 1))
              (`/Game/Interactables/BP_Shelf.UpdateAmount` (`self.shelfBP`))
              (goto _label_3)
              (elif (`/Game/Interactables/BP_Shelf.isTomato` _shelfbp_2)
                (set `self.tomatoAmount` (+ (`self.tomatoAmount`) 1))
                (set `self.itemsHeld` (+ (`self.itemsHeld`) 1))
                (`/Game/Interactables/BP_Shelf.UpdateAmount` (`self.shelfBP`))
                (goto _label_3)
                (else
                  (`KismetSystemLibrary.PrintString` "[BP_Customer] Pickup Item Is Fucked Up"))))))
        (:`==`
          (`self.PickAnother` :!label _label_5))
        (:`<`
          (goto _label_5))))))

(event `Checkout`
  ;[1 1 1] AI MoveTo Checkout
  (set `self.isMoving` true)
  (set `self.readyToCheckout` true)
  (bind _returnvalue (`GameplayStatics.GetActorOfClass` "/Game/Interactables/Till_BP.Till_BP_C"))
  (bind _returnvalue_2 (`self.K2_GetActorLocation` _returnvalue))
  (set `self.MoveToLocation` _returnvalue_2)
  (`|AIMoveTo` self _returnvalue_2 null
    (:`OnSuccess`
      (set `self.isMoving` false))
    (:`OnFail`
      (`self.Checkout`)
      (`self.AI MoveTo Failed`))))

(event `Leave`
  ;[1 1 1] AI MoveTo Customer Despawner
  (`/Engine/EditorBlueprintResources/StandardMacros.CompareInt` (`self.itemsHeld`)
    (:`>`
      (`self.Checkout`))
    (:`==`
      (set `self.isMoving` true :!label _label_6)
      (bind _returnvalue (`GameplayStatics.GetActorOfClass` "/Game/Characters/Customers/BP_CustomerSpawner.BP_CustomerSpawner_C"))
      (`/Game/Characters/Customers/BP_CustomerSpawner.SpawnCustomer` _returnvalue)
      (bind _returnvalue_2 (`GameplayStatics.GetActorOfClass` "/Game/Characters/Customers/BP_CustomerDespawner.BP_CustomerDespawner_C"))
      (bind _returnvalue_3 (`self.K2_GetActorLocation` _returnvalue_2))
      (set `self.MoveToLocation` _returnvalue_3)
      (`|AIMoveTo` self _returnvalue_3 null
        (:`OnFail`
          (`self.Leave`)
          (`self.AI MoveTo Failed`))))
    (:`<`
      (goto _label_6))))

(fn `UserConstructionScript`)