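; BP_Fred is a fisherman character that wanders between farm plots and keeps tallies of harvested crops.
; A looping timer, also fired at BeginPlay, calls MoveToPlot, which uses AI MoveTo toward a random BP_FarmPlot unless CanDeliver is set.
; HarvestCrop adds HarvestAmount to the lettuce, tomato or carrot count and flags that crop as held.
; Move success or failure is only printed, and no delivery logic appears here.
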(event `self.ReceiveBeginPlay`
  (`KismetSystemLibrary.K2_SetTimerDelegate` (delegate `MoveToPlot`) (`self.moveToDelay`) true)
  (`self.MoveToPlot`))

(event `MoveToPlot`
  (if (not (`self.canDeliver`))
    (bind _outactors (`GameplayStatics.GetAllActorsOfClass` "/Game/Interactables/BP_FarmPlot.BP_FarmPlot_C"))
    (bind _outitem (`KismetArrayLibrary.Array_Random` _outactors))
    (`|AIMoveTo` self (`self.K2_GetActorLocation` _outitem) _outitem 0.0 true
      (:`OnSuccess`
        (`KismetSystemLibrary.PrintString` "Fred: AI MoveTo Success" true true (struct :`G` 0.5 :`A` 1.0)))
      (:`OnFail`
        (`KismetSystemLibrary.PrintString` "Fred: AI MoveTo Fail" true true (struct :`R` 0.5 :`A` 1.0))))))

(event `/Game/Interactables/BPI_FarmPlot.HarvestCrop`
  (params (FarmPlotClass :type "/Game/Interactables/BP_FarmPlot Class Reference") (isLettuce :type Boolean) (isTomato :type Boolean) (isCarrot :type Boolean))
  (if isLettuce
    (set `self.lettuceAmount` (+ (`self.lettuceAmount`) (`self.harvestAmount`)))
    (set `self.hasLettuce` true)
    (elif isTomato
      (set `self.tomatoAmount` (+ (`self.tomatoAmount`) (`self.harvestAmount`)))
      (set `self.hasTomato` true)
      (elif isCarrot
        (set `self.carrotAmount` (+ (`self.carrotAmount`) (`self.harvestAmount`)))
        (set `self.hasCarrot` true)))))

(fn `UserConstructionScript`)