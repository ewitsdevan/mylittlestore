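; BP_Shelf is an interactable produce shelf that displays carrots, tomatoes or lettuce, chosen by boolean flags, on nine Paper2D sprites.
; BeginPlay sets each sprite's image and rotation for that type, and UpdateAmount shows only as many sprites as StockAmount.
; When BP_Player overlaps the trigger, RestockShelf recursively moves matching items from the player's counts into stock until the shelf holds nine or the player runs out.
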(event `self.ReceiveBeginPlay`
  (set `self.SpritesArray` (`|MakeArray` (`self.PaperSprite1`) (`self.PaperSprite2`) (`self.PaperSprite3`) (`self.PaperSprite4`) (`self.PaperSprite5`) (`self.PaperSprite6`) (`self.PaperSprite7`) (`self.PaperSprite8`) (`self.PaperSprite9`)))
  (if (`self.isCarrot`)
    (for _array_element (`self.SpritesArray`)
      (`PaperSpriteComponent.SetSprite` _array_element "/Game/2D_Assets/Vegtables/Carrot_SINGLE_Sprite.Carrot_SINGLE_Sprite")
      (`SceneComponent.K2_SetRelativeRotation` _array_element (struct :`Pitch` 45.0 :`Yaw` 40.0 :`Roll` -40.0) false false)
      (`self.UpdateAmount`))
    (elif (`self.isTomato`)
      (for _array_element_2 (`self.SpritesArray`)
        (`PaperSpriteComponent.SetSprite` _array_element_2 "/Game/2D_Assets/Vegtables/Tomato_SINGLE_Sprite.Tomato_SINGLE_Sprite")
        (`SceneComponent.K2_SetRelativeRotation` _array_element_2 (struct :`Pitch` -30.0 :`Yaw` 90.0 :`Roll` -45.0) false false)
        (`self.UpdateAmount`))
      (elif (`self.isLettuce`)
        (for _array_element_3 (`self.SpritesArray`)
          (`PaperSpriteComponent.SetSprite` _array_element_3 "/Game/2D_Assets/Vegtables/Lettuce_SINGLE_Sprite.Lettuce_SINGLE_Sprite")
          (`SceneComponent.K2_SetRelativeRotation` _array_element_3 (struct :`Pitch` -30.0 :`Yaw` 90.0 :`Roll` -45.0) false false)
          (`self.UpdateAmount`))))))

(event `UpdateAmount`
  (for (_array_element _array_index) (`self.SpritesArray`)
    (`/Engine/EditorBlueprintResources/StandardMacros.CompareInt` (+ _array_index 1) (`self.stockAmount`)
      (:`>`
        (`SceneComponent.SetVisibility` _array_element false false))
      (:`==`
        (`SceneComponent.SetVisibility` _array_element true false :!label _label))
      (:`<`
        (goto _label)))))

(event `self.Trigger.OnComponentBeginOverlap`
  (params (OverlappedComponent :type "PrimitiveComponent Object Reference") (OtherActor :type "Actor Object Reference") (OtherComp :type "PrimitiveComponent Object Reference") (OtherBodyIndex :type Integer) (bFromSweep :type Boolean) (SweepResult :type "HitResult Structure (by ref)"))
  (set `self.Other Actor` OtherActor)
  (if (`KismetMathLibrary.ClassIsChildOf` (`GameplayStatics.GetObjectClass` OtherActor) "/Game/Characters/Player/BP_Player.BP_Player_C")
    (bind _asbp_player (cast `/Game/Characters/Player/BP_Player` (`self.Other Actor`)))
    (set `self.playerBP` _asbp_player)
    (`self.RestockShelf`)))

(event `RestockShelf`
  (bind _playerbp (`self.playerBP`))
  (bind _playerbp_2 (`self.playerBP`))
  (bind _playerbp_3 (`self.playerBP`))
  (`/Engine/EditorBlueprintResources/StandardMacros.CompareInt` (`self.stockAmount`) 9
    (:`<`
      (if (`self.isCarrot`)
        (`/Engine/EditorBlueprintResources/StandardMacros.CompareInt` (`/Game/Characters/Player/BP_Player.carrotAmount` (`self.playerBP`))
          (:`>`
            (set `self.stockAmount` (+ (`self.stockAmount`) 1))
            (set `/Game/Characters/Player/BP_Player.carrotAmount` (- (`/Game/Characters/Player/BP_Player.carrotAmount` _playerbp_2) 1) _playerbp_2)
            (`self.UpdateAmount` :!label _label_2)
            (`self.RestockShelf`)))
        (elif (`self.isTomato`)
          (`/Engine/EditorBlueprintResources/StandardMacros.CompareInt` (`/Game/Characters/Player/BP_Player.tomatoAmount` (`self.playerBP`))
            (:`>`
              (set `self.stockAmount` (+ (`self.stockAmount`) 1))
              (set `/Game/Characters/Player/BP_Player.tomatoAmount` (- (`/Game/Characters/Player/BP_Player.tomatoAmount` _playerbp_3) 1) _playerbp_3)
              (goto _label_2)))
          (elif (`self.isLettuce`)
            (`/Engine/EditorBlueprintResources/StandardMacros.CompareInt` (`/Game/Characters/Player/BP_Player.lettuceAmount` (`self.playerBP`))
              (:`>`
                (set `self.stockAmount` (+ (`self.stockAmount`) 1))
                (set `/Game/Characters/Player/BP_Player.lettuceAmount` (- (`/Game/Characters/Player/BP_Player.lettuceAmount` _playerbp) 1) _playerbp)
                (goto _label_2)))))))))

(fn `UserConstructionScript`)