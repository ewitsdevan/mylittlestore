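; BP_FarmPlot is an interactable crop plot that regrows on a timer and is harvested when an actor walks into it.
; ResetPlot shows the growing plant and starts a ten-second timer that swaps to the harvestable plant.
; Overlapping actors implementing BPI_FarmPlot receive a harvest message with the plot class and crop-type flags, then the plot resets.
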(event `self.ReceiveBeginPlay`
  (`self.Reset Plot`))

(event `self.Box.OnComponentBeginOverlap`
  (params (OverlappedComponent :type "PrimitiveComponent Object Reference") (OtherActor :type "Actor Object Reference") (OtherComp :type "PrimitiveComponent Object Reference") (OtherBodyIndex :type Integer) (bFromSweep :type Boolean) (SweepResult :type "HitResult Structure (by ref)"))
  (set `self.Other Actor` OtherActor)
  (if (`KismetSystemLibrary.DoesImplementInterface` OtherActor "/Game/Interactables/BPI_FarmPlot.BPI_FarmPlot_C")
    (if (`self.isHarvestable`)
      (message `/Game/Interactables/BPI_FarmPlot.HarvestCrop` (`self.Other Actor`) (`GameplayStatics.GetObjectClass` self) (`self.isLettuce`) (`self.isTomato`) (`self.isCarrot`))
      (`self.Reset Plot`))))

(event `Reset Plot`
  (set `self.isHarvestable` false)
  (`SceneComponent.SetVisibility` (`self.GrowingPlant`) true false)
  (`SceneComponent.SetVisibility` (`self.HarvestablePlant`) false false)
  (`KismetSystemLibrary.K2_SetTimerDelegate` (delegate `Harvestable`) 10.0))

(event `Harvestable`
  (set `self.isHarvestable` true)
  (`SceneComponent.SetVisibility` (`self.GrowingPlant`) false false)
  (`SceneComponent.SetVisibility` (`self.HarvestablePlant`) true false))

(fn `UserConstructionScript`)