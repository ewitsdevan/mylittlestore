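; Shop till that checks out customers and holds their payments until the player collects them.
; Overlap events track the player and ready customers, who wait unless checkout is enabled by the player or an unlocked employee.
; Checkout totals produce and fish prices, doubled with donations unlocked, pays a present player or banks it, then dismisses the customer.
; Sales and collections trigger chained open and close drawer timelines with sounds.
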(event `RegisterAnimation`
  (bind (_relativelocation_x _relativelocation_y _relativelocation_z) (`KismetMathLibrary.BreakVector` (`SceneComponent.RelativeLocation` (`self.Till_DRAWER`))))
  ;[1 1 1] Register Drawer Animation
  (if (`self.canAnimate`)
    (set `self.canAnimate` false)
    (`GameplayStatics.PlaySoundAtLocation` "/Game/Audio/SFX/WAVS/Till_Open.Till_Open" (`self.K2_GetActorLocation` self) (struct) 1.0 1.0 0.0 null null null)
    (set `self.Drawer_StartLOC` (`KismetMathLibrary.MakeVector` _relativelocation_x _relativelocation_y _relativelocation_z))
    (set `self.Drawer_EndLOC` (`KismetMathLibrary.MakeVector` (+ _relativelocation_x 30.0) _relativelocation_y _relativelocation_z))
    (bind (_direction _draweropen) (`Timeline|Open Drawer` :!via `PlayFromStart`)
      (:`Update`
        (`SceneComponent.K2_SetRelativeLocation` (`self.Till_DRAWER`) (`KismetMathLibrary.VLerp` (`self.Drawer_StartLOC`) (`self.Drawer_EndLOC`) _draweropen) false false))
      (:`Finished`
        (`self.CloseRegister`)))))

(event `CloseRegister`
  (bind (_relativelocation_x _relativelocation_y _relativelocation_z) (`KismetMathLibrary.BreakVector` (`SceneComponent.RelativeLocation` (`self.Till_DRAWER`))))
  ;[1 1 1] Register Drawer Animation
  (`KismetSystemLibrary.Delay` 1.0)
  (`GameplayStatics.PlaySoundAtLocation` "/Game/Audio/SFX/WAVS/Till_Closed.Till_Closed" (`self.K2_GetActorLocation` self) (struct) 1.0 1.0 0.0 null null null)
  (set `self.Drawer_StartLOC` (`KismetMathLibrary.MakeVector` _relativelocation_x _relativelocation_y _relativelocation_z))
  (set `self.Drawer_EndLOC` (`KismetMathLibrary.MakeVector` (+ _relativelocation_x -30.0) _relativelocation_y _relativelocation_z))
  (bind (_direction _draweropen) (`Timeline|Close Drawer` :!via `PlayFromStart`)
    (:`Update`
      (`SceneComponent.K2_SetRelativeLocation` (`self.Till_DRAWER`) (`KismetMathLibrary.VLerp` (`self.Drawer_StartLOC`) (`self.Drawer_EndLOC`) _draweropen) false false))
    (:`Finished`
      (set `self.canAnimate` true))))

(event `self.PlayerCOLLECT.OnComponentBeginOverlap`
  (params (OverlappedComponent :type "PrimitiveComponent Object Reference") (OtherActor :type "Actor Object Reference") (OtherComp :type "PrimitiveComponent Object Reference") (OtherBodyIndex :type Integer) (bFromSweep :type Boolean) (SweepResult :type "HitResult Structure (by ref)"))
  ;[1 1 1] Player Collect & Checkout
  (set `self.registerActor` OtherActor)
  (if (`KismetMathLibrary.ClassIsChildOf` (`GameplayStatics.GetObjectClass` OtherActor) "/Game/Characters/Player/BP_Player.BP_Player_C")
    (bind _asbp_player (cast `/Game/Characters/Player/BP_Player` (`self.registerActor`)))
    (set `self.playerBP` _asbp_player)
    (`/Engine/EditorBlueprintResources/StandardMacros.CompareInt` (`self.MoneyInTILL`)
      (:`>`
        (`/Game/Characters/Player/BP_Player.PlayerCollected` (`self.playerBP`) (`self.MoneyInTILL`))
        (`self.RegisterAnimation`)
        (set `self.MoneyInTILL` 0)
        (bind _asmoney_widget (cast `/Game/UI/Widgets/MoneyWIDGET` (`WidgetComponent.GetWidget` (`self.MoneyICON`))))
        (`/Game/UI/Widgets/MoneyWIDGET.GotMoney ANIM` _asmoney_widget)
        (set `self.canCheckout` true)
        (set `self.playerCheckout` true)
        (if (`self.isCustomerWaiting`)
          (`self.CheckoutCustomer`)))
      (:`<`
        (set `self.playerCheckout` true)
        (if (not (`self.employeeUnlocked`))
          (set `self.canCheckout` true))
        (if (`self.isCustomerWaiting`)
          (`self.CheckoutCustomer`))))))

(event `self.ReceiveActorEndOverlap`
  (params (OtherActor :type "Actor Object Reference"))
  ;[1 1 1] Player Collect & Checkout
  (if (`KismetMathLibrary.ClassIsChildOf` (`GameplayStatics.GetObjectClass` OtherActor) "/Game/Characters/Player/BP_Player.BP_Player_C")
    (set `self.playerCheckout` false)
    (if (not (`self.employeeUnlocked`))
      (set `self.canCheckout` false))))

(event `UnlockEmployee`
  ;[1 1 1] Unlock Employee
  (`SceneComponent.SetHiddenInGame` (`self.Employee`) false false)
  (set `self.employeeUnlocked` true)
  (set `self.canCheckout` true))

(event `self.CustomerCheckout.OnComponentBeginOverlap`
  (params (OverlappedComponent :type "PrimitiveComponent Object Reference") (OtherActor :type "Actor Object Reference") (OtherComp :type "PrimitiveComponent Object Reference") (OtherBodyIndex :type Integer) (bFromSweep :type Boolean) (SweepResult :type "HitResult Structure (by ref)"))
  ;[1 1 1] Customer At Checkout
  (bind _output_get (set `self.checkoutActor` OtherActor))
  (bind _asbp_customer (cast `/Game/Characters/Customers/BP_Customer` _output_get))
  (bind _output_get_2 (set `self.customerBP` _asbp_customer))
  (if (`/Game/Characters/Customers/BP_Customer.readyToCheckout` _output_get_2)
    (if (`self.canCheckout`)
      (`self.CheckoutCustomer`)
      (else
        (set `self.isCustomerWaiting` true)))))

(event `self.CustomerCheckout.OnComponentEndOverlap`
  (params (OverlappedComponent :type "PrimitiveComponent Object Reference") (OtherActor :type "Actor Object Reference") (OtherComp :type "PrimitiveComponent Object Reference") (OtherBodyIndex :type Integer))
  ;[1 1 1] Customer At Checkout
  (cast `/Game/Characters/Customers/BP_Customer` OtherActor)
  (set `self.isCustomerWaiting` false))

(event `CheckoutCustomer`
  (bind _returnvalue (+ (* (`/Game/Characters/Customers/BP_Customer.tomatoAmount` (`self.customerBP`)) (`self.tomatoPrice`)) (* (`/Game/Characters/Customers/BP_Customer.lettuceAmount` (`self.customerBP`)) (`self.lettucePrice`)) (* (`/Game/Characters/Customers/BP_Customer.carrotAmount` (`self.customerBP`)) (`self.carrotPrice`)) (* (`/Game/Characters/Customers/BP_Customer.fishAmount` (`self.customerBP`)) (`self.fishPrice`))))
  ;[1 1 1] Checkout Customer
  (if (`self.donationsUnlocked`)
    (set `self.collectAmount` (* _returnvalue 2))
    (else
      (set `self.collectAmount` _returnvalue)))
  (if (`self.playerCheckout`)
    (`/Game/Characters/Player/BP_Player.PlayerCollected` (`self.playerBP`) (`self.collectAmount`))
    (set `self.collectAmount` 0)
    (else
      (set `self.MoneyInTILL` (+ (`self.MoneyInTILL`) (`self.collectAmount`)))
      (set `self.collectAmount` 0)))
  (set `/Game/Characters/Customers/BP_Customer.itemsHeld` 0 (`self.customerBP`))
  (`/Game/Characters/Customers/BP_Customer.Leave` (`self.customerBP`))
  (`self.RegisterAnimation`))

(fn `Interact`
  (params (Player :type "/Game/Characters/Player/BP_Player Object Reference"))
  (returns (Success :type Boolean))
  (return false))

(fn `UserConstructionScript`)