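; BP_Fridge is an interactable fridge that stores up to six fish taken from the player's carried supply.
; When a BP_Player overlaps its Trigger, RestockFridge recursively moves one fish at a time from the player's FishAmount into StockAmount until it is full or the player runs out.
; Each transfer calls UpdateAmount, also run at BeginPlay, which shows as many of the six paper sprites as there are fish in stock.
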(event `self.ReceiveBeginPlay`
  (set `self.SpritesArray` (`|MakeArray` (`self.PaperSprite1`) (`self.PaperSprite2`) (`self.PaperSprite3`) (`self.PaperSprite4`) (`self.PaperSprite5`) (`self.PaperSprite6`)))
  (`self.UpdateAmount`))

(event `UpdateAmount`
  (for (_array_element _array_index) (`self.SpritesArray`)
    (`/Engine/EditorBlueprintResources/StandardMacros.CompareInt` (+ _array_index 1) (`self.stockAmount`)
      (:`>`
        (`SceneComponent.SetVisibility` _array_element false false))
      (:`==`
        (`SceneComponent.SetVisibility` _array_element true false :!label _label))
      (:`<`
        (goto _label)))))

(event `self.Trigger.OnComponentBeginOverlap`
  (params (OverlappedComponent :type "PrimitiveComponent Object Reference") (OtherActor :type "Actor Object Reference") (OtherComp :type "PrimitiveComponent Object Reference") (OtherBodyIndex :type Integer) (bFromSweep :type Boolean) (SweepResult :type "HitResult Structure (by ref)"))
  (set `self.Other Actor` OtherActor)
  (if (`KismetMathLibrary.ClassIsChildOf` (`GameplayStatics.GetObjectClass` OtherActor) "/Game/Characters/Player/BP_Player.BP_Player_C")
    (bind _asbp_player (cast `/Game/Characters/Player/BP_Player` (`self.Other Actor`)))
    (set `self.playerBP` _asbp_player)
    (`self.Restock Fridge`)))

(event `Restock Fridge`
  (bind _playerbp (`self.playerBP`))
  (`/Engine/EditorBlueprintResources/StandardMacros.CompareInt` (`self.stockAmount`) 6
    (:`<`
      (`/Engine/EditorBlueprintResources/StandardMacros.CompareInt` (`/Game/Characters/Player/BP_Player.fishAmount` (`self.playerBP`))
        (:`>`
          (set `self.stockAmount` (+ (`self.stockAmount`) 1))
          (set `/Game/Characters/Player/BP_Player.fishAmount` (- (`/Game/Characters/Player/BP_Player.fishAmount` _playerbp) 1) _playerbp)
          (`self.UpdateAmount`)
          (`self.Restock Fridge`))))))

(fn `UserConstructionScript`)