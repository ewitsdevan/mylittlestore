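; BP_DeliveryBox is an interactable drop-off box that relays produce from BP_BenFarmer to BP_Player.
; When the farmer overlaps the Collider carrying items, the box adds his lettuce, tomato and carrot counts to its own and resets his items.
; When the player overlaps a filled box, it passes the totals to CollectDelivery and resets.
; Fish is passed along but never incremented, and the closed mesh is never shown.
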(event `self.ReceiveBeginPlay`
  (`self.ResetBox`))

(event `ResetBox`
  (set `self.lettuceAmount` 0)
  (set `self.tomatoAmount` 0)
  (set `self.carrotAmount` 0)
  (set `self.fishAmount` 0)
  (set `self.hasItems` false)
  (`SceneComponent.SetVisibility` (`self.BoxClosed`) false false)
  (`SceneComponent.SetVisibility` (`self.BoxOpen`) true false))

(event `self.Collider.OnComponentBeginOverlap`
  (params (OverlappedComponent :type "PrimitiveComponent Object Reference") (OtherActor :type "Actor Object Reference") (OtherComp :type "PrimitiveComponent Object Reference") (OtherBodyIndex :type Integer) (bFromSweep :type Boolean) (SweepResult :type "HitResult Structure (by ref)"))
  (set `self.Other Actor` OtherActor)
  (if (`KismetMathLibrary.ClassIsChildOf` (`GameplayStatics.GetObjectClass` (`self.Other Actor`)) "/Game/Characters/Ben_Farmer/BP_BenFarmer.BP_BenFarmer_C")
    (bind _asbp_ben_farmer (cast `/Game/Characters/Ben_Farmer/BP_BenFarmer` (`self.Other Actor`)))
    (bind _output_get (set `self.BenBP` _asbp_ben_farmer))
    (`/Engine/EditorBlueprintResources/StandardMacros.CompareInt` (`/Game/Characters/Ben_Farmer/BP_BenFarmer.itemsTotal` _output_get)
      (:`>`
        (set `self.hasItems` true)
        (set `self.lettuceAmount` (+ (`/Game/Characters/Ben_Farmer/BP_BenFarmer.lettuceAmount` (`self.BenBP`)) (`self.lettuceAmount`)))
        (set `self.tomatoAmount` (+ (`/Game/Characters/Ben_Farmer/BP_BenFarmer.tomatoAmount` (`self.BenBP`)) (`self.tomatoAmount`)))
        (set `self.carrotAmount` (+ (`/Game/Characters/Ben_Farmer/BP_BenFarmer.carrotAmount` (`self.BenBP`)) (`self.carrotAmount`)))
        (`/Game/Characters/Ben_Farmer/BP_BenFarmer.ResetItems` (`self.BenBP`))))
    (elif (`KismetMathLibrary.ClassIsChildOf` (`GameplayStatics.GetObjectClass` (`self.Other Actor`)) "/Game/Characters/Player/BP_Player.BP_Player_C")
      (if (`self.hasItems`)
        (bind _asbp_player (cast `/Game/Characters/Player/BP_Player` (`self.Other Actor`)))
        (`/Game/Characters/Player/BP_Player.CollectDelivery` _asbp_player (`self.lettuceAmount`) (`self.tomatoAmount`) (`self.carrotAmount`) (`self.fishAmount`))
        (`self.ResetBox`)))))

(fn `UserConstructionScript`)