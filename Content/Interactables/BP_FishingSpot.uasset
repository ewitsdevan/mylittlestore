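; BP_FishingSpot is an interactable that marks an area where the player can fish.
; Its Collider sets CanFish on an overlapping BP_Player to true on entry and false on exit.
; A separate InteractWIDGET overlap volume calls InteractIN and InteractOUT on the Interaction_Widget to toggle the interaction prompt as the player enters and leaves.
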(event `self.Collider.OnComponentBeginOverlap`
  (params (OverlappedComponent :type "PrimitiveComponent Object Reference") (OtherActor :type "Actor Object Reference") (OtherComp :type "PrimitiveComponent Object Reference") (OtherBodyIndex :type Integer) (bFromSweep :type Boolean) (SweepResult :type "HitResult Structure (by ref)"))
  (bind _output_get (set `self.Other Actor` OtherActor))
  (bind _asbp_player (cast `/Game/Characters/Player/BP_Player` _output_get))
  (set `/Game/Characters/Player/BP_Player.canFish` true _asbp_player))

(event `self.Collider.OnComponentEndOverlap`
  (params (OverlappedComponent :type "PrimitiveComponent Object Reference") (OtherActor :type "Actor Object Reference") (OtherComp :type "PrimitiveComponent Object Reference") (OtherBodyIndex :type Integer))
  (bind _output_get (set `self.Other Actor` OtherActor))
  (bind _asbp_player (cast `/Game/Characters/Player/BP_Player` _output_get))
  (set `/Game/Characters/Player/BP_Player.canFish` false _asbp_player))

(event `self.InteractWIDGET.OnComponentBeginOverlap`
  (params (OverlappedComponent :type "PrimitiveComponent Object Reference") (OtherActor :type "Actor Object Reference") (OtherComp :type "PrimitiveComponent Object Reference") (OtherBodyIndex :type Integer) (bFromSweep :type Boolean) (SweepResult :type "HitResult Structure (by ref)"))
  ;[1 1 1] Interact Widget
  (cast `/Game/Characters/Player/BP_Player` OtherActor)
  (bind _asinteraction_widget (cast `/Game/UI/Player/Interaction_Widget` (`WidgetComponent.GetWidget` (`self.InteractionWidget`))))
  (`/Game/UI/Player/Interaction_Widget.InteractIN` _asinteraction_widget))

(event `self.InteractWIDGET.OnComponentEndOverlap`
  (params (OverlappedComponent :type "PrimitiveComponent Object Reference") (OtherActor :type "Actor Object Reference") (OtherComp :type "PrimitiveComponent Object Reference") (OtherBodyIndex :type Integer))
  ;[1 1 1] Interact Widget
  (cast `/Game/Characters/Player/BP_Player` OtherActor)
  (`/Game/UI/Player/Interaction_Widget.InteractOUT` (stale `self.InteractWIDGET.OnComponentBeginOverlap` _asinteraction_widget)))

(fn `UserConstructionScript`)