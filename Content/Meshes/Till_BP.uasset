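; Cash till that accrues money roughly every two seconds through test Tick logic and lets the player collect it by walking up.
; Overlapping the collect component notifies BP_Player, zeroes the till, plays a sound and animates the money widget.
; Timelines lerp the drawer open on collection and closed, with sound, when the player leaves, using offsets from its current relative position.
; Interact is a stub returning false.
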(event `self.ReceiveTick`
  (params (DeltaSeconds :type "Float (single-precision)"))
  ;[1 0 0.04868] Testing
  (`KismetSystemLibrary.Delay` 2.0)
  (set `self.MoneyInTILL` (+ (`self.MoneyInTILL`) (`self.MoneyComingIN`))))

(event `self.PlayerCOLLECT.OnComponentBeginOverlap`
  (params (OverlappedComponent :type "PrimitiveComponent Object Reference") (OtherActor :type "Actor Object Reference") (OtherComp :type "PrimitiveComponent Object Reference") (OtherBodyIndex :type Integer) (bFromSweep :type Boolean) (SweepResult :type "HitResult Structure (by ref)"))
  ;[1 1 1] Player Collects Money
  (bind _asbp_player (cast `/Game/Characters/Player/BP_Player` OtherActor))
  (`/Game/Characters/Player/BP_Player.PlayerCollected` _asbp_player)
  (`self.TillAnimationOPEN`)
  (`GameplayStatics.PlaySoundAtLocation` "/Game/Audio/SFX/WAVS/Till_Open.Till_Open" (`self.K2_GetActorLocation` self) (struct) 1.0 1.0 0.0 null null null)
  (set `self.MoneyInTILL` 0)
  (bind _asmoney_widget (cast `/Game/UI/Widgets/MoneyWIDGET` (`WidgetComponent.GetWidget` (`self.MoneyICON`))))
  (`/Game/UI/Widgets/MoneyWIDGET.GotMoney ANIM` _asmoney_widget))

(event `self.ReceiveActorEndOverlap`
  (params (OtherActor :type "Actor Object Reference"))
  ;[1 1 1] Player Collects Money
  (cast `/Game/Characters/Player/BP_Player` OtherActor)
  (`self.TillAnimationCLOSE`)
  (`GameplayStatics.PlaySoundAtLocation` "/Game/Audio/SFX/WAVS/Till_Closed.Till_Closed" (`self.K2_GetActorLocation` self) (struct) 1.0 1.0 0.0 null null null))

(event `TillAnimationOPEN`
  (bind (_relativelocation_x _relativelocation_y _relativelocation_z) (`KismetMathLibrary.BreakVector` (`SceneComponent.RelativeLocation` (`self.Till_DRAWER`))))
  ;[1 1 1] Till Drawer Animation
  (if (`self.DrawerOpen?`)
    (`KismetSystemLibrary.Delay` 0.5))
  (set `self.Drawer_StartLOC` (`KismetMathLibrary.MakeVector` _relativelocation_x _relativelocation_y _relativelocation_z))
  (set `self.Drawer_EndLOC` (`KismetMathLibrary.MakeVector` (+ _relativelocation_x 30.0) _relativelocation_y _relativelocation_z))
  (bind (_direction _draweropen) (`Timeline|Open Drawer` :!via `PlayFromStart`)
    (:`Update`
      (`SceneComponent.K2_SetRelativeLocation` (`self.Till_DRAWER`) (`KismetMathLibrary.VLerp` (`self.Drawer_StartLOC`) (`self.Drawer_EndLOC`) _draweropen) false false)
      (set `self.DrawerOpen?` true))))

(event `TillAnimationCLOSE`
  (bind (_relativelocation_x _relativelocation_y _relativelocation_z) (`KismetMathLibrary.BreakVector` (`SceneComponent.RelativeLocation` (`self.Till_DRAWER`))))
  ;[1 1 1] Till Drawer Animation
  (if (not (`self.DrawerOpen?`))
    (`KismetSystemLibrary.Delay` 0.5))
  (set `self.Drawer_StartLOC` (`KismetMathLibrary.MakeVector` _relativelocation_x _relativelocation_y _relativelocation_z))
  (set `self.Drawer_EndLOC` (`KismetMathLibrary.MakeVector` (+ _relativelocation_x -30.0) _relativelocation_y _relativelocation_z))
  (bind (_direction _draweropen) (`Timeline|Close Drawer` :!via `PlayFromStart`)
    (:`Update`
      (`SceneComponent.K2_SetRelativeLocation` (`self.Till_DRAWER`) (`KismetMathLibrary.VLerp` (`self.Drawer_StartLOC`) (`self.Drawer_EndLOC`) _draweropen) false false)
      (set `self.DrawerOpen?` false))))

(fn `Interact`
  (params (Player :type "/Game/Characters/Player/BP_Player Object Reference"))
  (returns (Success :type Boolean))
  (return false))

(fn `UserConstructionScript`)