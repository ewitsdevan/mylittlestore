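; BP_Boat is an environment boat that gently rocks once play begins.
; On BeginPlay it caches the mesh's relative rotation and a target offset by a few degrees on roll, pitch and yaw; despite the LOC names, both hold rotations.
; The BoatRocking timeline then drives a rotator lerp between the two, applied to BoatMESH on each update.
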(event `self.ReceiveBeginPlay`
  (bind (_relativerotation_roll _relativerotation_pitch _relativerotation_yaw) (`KismetMathLibrary.BreakRotator` (`SceneComponent.RelativeRotation` (`self.Boat_MESH`))))
  (set `self.StartLOC` (`KismetMathLibrary.MakeRotator` _relativerotation_roll _relativerotation_pitch _relativerotation_yaw))
  (set `self.EndLOC` (`KismetMathLibrary.MakeRotator` (+ _relativerotation_roll 5.0) (+ _relativerotation_pitch 5.0) (+ _relativerotation_yaw 5.0)))
  (bind (_direction _rocking) (`Timeline|Boat Rocking` :!via `PlayFromStart`)
    (:`Update`
      (`SceneComponent.K2_SetRelativeRotation` (`self.Boat_MESH`) (`KismetMathLibrary.RLerp` (`self.StartLOC`) (`self.EndLOC`) _rocking) false false))))

(fn `UserConstructionScript`)